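; Boss character for root-motion combat that always faces the RootMotionTestDummy player and exposes move, dodge, attack and special-hit events.
; Move events set target axes, which Tick smooths into clamped final axis values.
; Dodge picks a directional roll from those targets; Attack plays a random montage with matching damage, using Flying mode and mutual action locks.
; Notify windows gate capsule-overlap damage to the player; example behaviour sequence is unconnected.
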(event `MoveRight`
  ;[1 0.8341 0] Root motion locomotion
  ;;[0 0 0] (IMPORTANT VARIABLES)                            Target X = Right (1) Left (-1)                                                          Target Y = Forward (1) Backward (-1)             Move Boss? Should be set true when you want to move the boss, false when you want the boss to stop moving. Example
  ;;;[0 1 0.06186] Move Right
  (set `self.TargetX` 1.0)
  (set `self.MoveBoss?` true))

(event `self.ReceiveTick`
  (params (DeltaSeconds :type "Float (single-precision)"))
  (bind _returnvalue (`KismetMathLibrary.Lerp` (`self.CurrentY`) (`self.TargetY`) 0.1))
  (bind _returnvalue_2 (`KismetMathLibrary.Lerp` (`self.CurrentX`) (`self.TargetX`) 0.1))
  (bind (_returnvalue_roll _returnvalue_pitch _returnvalue_yaw) (`KismetMathLibrary.BreakRotator` (`KismetMathLibrary.FindLookAtRotation` (`SceneComponent.K2_GetComponentLocation` (`self.CapsuleComponent`)) (`self.K2_GetActorLocation` (`self.As Root Motion Test Dummy`)))))
  ;[1 0.8341 0] Root motion locomotion
  ;;[1 0.696 0.1385] Root motion engine
  (if (`self.MoveBoss?`)
    (set `self.Moving?` true)
    (if (`self.Moving?`)
      (`|ExecutionSequence` :!label _label
        (:`then_0`
          (set `self.CurrentX` _returnvalue_2)
          (set `self.XAxisFinal` (`KismetMathLibrary.FClamp` _returnvalue_2 -1.0)))
        (:`then_1`
          (set `self.CurrentY` _returnvalue)
          (set `self.YAxisFinal` (`KismetMathLibrary.FClamp` _returnvalue -1.0))
          (if (not (== (== (`self.XAxisFinal`) 0.0) (== (`self.YAxisFinal`) 0.0)))
            (set `self.Moving?` false)))
        (:`then_2`
          (`self.K2_SetActorRotation` self (`KismetMathLibrary.MakeRotator` 0.0 0.0 _returnvalue_yaw) false))))
    (else
      (goto _label))))

(event `StopMoving`
  ;[1 0.8341 0] Root motion locomotion
  ;;[0 0 0] (IMPORTANT VARIABLES)                            Target X = Right (1) Left (-1)                                                          Target Y = Forward (1) Backward (-1)             Move Boss? Should be set true when you want to move the boss, false when you want the boss to stop moving. Example
  ;;;[1 0 0.02173] Stop Moving
  (set `self.TargetX` 0.0)
  (set `self.TargetY` 0.0)
  (set `self.MoveBoss?` false))

(event `MoveLeft`
  ;[1 0.8341 0] Root motion locomotion
  (set `self.TargetX` -1.0)
  (set `self.MoveBoss?` true))

(event `MoveForward`
  ;[1 0.8341 0] Root motion locomotion
  (set `self.TargetY` 1.0)
  (set `self.MoveBoss?` true))

(event `MoveBackwards`
  ;[1 0.8341 0] Root motion locomotion
  (set `self.TargetY` -1.0)
  (set `self.MoveBoss?` true))

(event `Dodge`
  (bind (_x _y) (`KismetMathLibrary.BreakVector2D` (`KismetMathLibrary.MakeVector2D` (`self.TargetX`) (`self.TargetY`))))
  ;[1 1 1] Dodge
  (if (`self.CanDodge?`)
    (set `self.CanAttack?` false)
    (set `self.CanDodge?` false)
    ;;[0.4747 1 0.2734] W A S D
    (if (>= _y 0.1)
      (set `self.DashValue` 0 :!label _label_2)
      (elif (<= _x -0.1)
        (set `self.DashValue` 1)
        (elif (<= _y -0.1)
          (set `self.DashValue` 2)
          (elif (>= _x 0.1)
            (set `self.DashValue` 3)
            (else
              (goto _label_2))))))
    (`|PlayMontage` (`self.Mesh`) (select `int` (`self.DashValue`) :`0` "/Game/CharacterTestPrototype/HighQualityMaleFolder/HumanMaleHighQualityAnimsFolder/Pass_1_roll_Montage.Pass_1_roll_Montage" :`1` "/Game/CharacterTestPrototype/HighQualityMaleFolder/HumanMaleHighQualityAnimsFolder/Pass_1_roll1_Montage.Pass_1_roll1_Montage" :`2` "/Game/CharacterTestPrototype/HighQualityMaleFolder/HumanMaleHighQualityAnimsFolder/Pass_1_roll3_Montage.Pass_1_roll3_Montage" :`3` "/Game/CharacterTestPrototype/HighQualityMaleFolder/HumanMaleHighQualityAnimsFolder/Pass_1_roll2_Montage.Pass_1_roll2_Montage" :!type "AnimMontage Object Reference")
      (:`OnCompleted`
        (set `self.CanDodge?` true)
        (set `self.CanAttack?` true)))))

(event `self.ReceiveBeginPlay`
  ;[0.1366 0.04973 1] Can be inherited from game manager
  (bind _returnvalue (`GameplayStatics.GetActorOfClass` "/Game/CharacterTestPrototype/RootMotionTestDummy.RootMotionTestDummy_C"))
  (set `self.As Root Motion Test Dummy` _returnvalue))

(event `self.ReceiveAnyDamage`
  (params (Damage :type "Float (single-precision)") (DamageType :type "DamageType Object Reference") (InstigatedBy :type "Controller Object Reference") (DamageCauser :type "Actor Object Reference"))
  ;[1 1 1] Apply damage to boss
  (bind _output_get (set `self.enemy_health` (- (`self.enemy_health`) Damage)))
  (`KismetSystemLibrary.PrintString` "New Boss Hp" true true (struct :`R` 1.0 :`G` 0.0409 :`A` 1.0))
  (`KismetSystemLibrary.PrintString` (`KismetStringLibrary.Conv_DoubleToString` _output_get) true true (struct :`R` 1.0 :`G` 0.0409 :`A` 1.0)))

(event `self.Capsule.OnComponentBeginOverlap`
  (params (OverlappedComponent :type "PrimitiveComponent Object Reference") (OtherActor :type "Actor Object Reference") (OtherComp :type "PrimitiveComponent Object Reference") (OtherBodyIndex :type Integer) (bFromSweep :type Boolean) (SweepResult :type "HitResult Structure (by ref)"))
  ;[1 1 1] Apply damage to player
  (if (`KismetStringLibrary.EqualEqual_StrStr` (`KismetSystemLibrary.GetDisplayName` OtherActor) "RootMotionTestDummy0")
    (if (`self.CanHitPlayer?`)
      (`KismetSystemLibrary.PrintString` (`KismetSystemLibrary.GetDisplayName` OtherActor))
      (set `self.CanHitPlayer?` false)
      (`GameplayStatics.ApplyDamage` (`self.As Root Motion Test Dummy`) (`self.BossCurrentDamage`)))))

(event `Attack`
  (bind _charactermovement (`self.CharacterMovement`))
  ;[1 1 1] Attack
  (if (`self.CanAttack?`)
    (set `self.CanDodge?` false)
    (set `self.CanAttack?` false)
    (bind _returnvalue (`self.DamageSystem`))
    (`CharacterMovementComponent.SetMovementMode` _charactermovement "MOVE_Flying" 0)
    (bind _notifyname (`|PlayMontage` (`self.Mesh`) _returnvalue)
      (:`OnCompleted`
        (set `self.CanAttack?` true)
        (set `self.CanDodge?` true)
        (`CharacterMovementComponent.SetMovementMode` _charactermovement "MOVE_Walking" 0))
      (:`OnNotifyBegin`
        (bind _returnvalue_2 (== _notifyname "HitDetectionAnimNotify"))
        (if _returnvalue_2
          (set `self.CanHitPlayer?` true)
          (`KismetSystemLibrary.PrintString` "CanHitPlayer" true true (struct :`R` 1.0 :`B` 0.047211 :`A` 1.0))))
      (:`OnNotifyEnd`
        (if _returnvalue_2
          (set `self.CanHitPlayer?` false)
          (`KismetSystemLibrary.PrintString` "CantHitPlayer" true true (struct :`R` 1.0 :`B` 0.047211 :`A` 1.0)))))))

(event `HitBySpecial`
  (params (SpecialType :type Integer))
  (switch `int` SpecialType
    (:`0`
      (`|PlayMontage` (`self.Mesh`) "/Game/CharacterTestPrototype/HighQualityMaleFolder/HumanMaleHighQualityAnimsFolder/BossGettingHitBySpecial1_Montage.BossGettingHitBySpecial1_Montage"
        (:`OnCompleted`
          (`GameplayStatics.ApplyDamage` self 100.0))))))

(fn `DamageSystem`
  (returns (ReturnValue :type "AnimMontage Object Reference"))
  ;[1 0.7982 0.8167] Damage system : The integer will determine which attack to play, along with how much damage that attack should deal.
  (set `self.SelectedAttack` (`KismetMathLibrary.RandomIntegerInRange` 0 2))
  (switch `int` (`self.SelectedAttack`)
    (:`0`
      (set `self.BossCurrentDamage` 25.0))
    (:`1`
      (set `self.BossCurrentDamage` 22.0))
    (:`2`
      (set `self.BossCurrentDamage` 35.0)))
  (return (select `int` (`self.SelectedAttack`) :`0` "/Game/CharacterTestPrototype/HighQualityMaleFolder/HumanMaleHighQualityAnimsFolder/Attack_anim_pass_1_Montage.Attack_anim_pass_1_Montage" :`1` "/Game/CharacterTestPrototype/HighQualityMaleFolder/HumanMaleHighQualityAnimsFolder/Attack_anim_pass_2_Montage.Attack_anim_pass_2_Montage" :`2` "/Game/CharacterTestPrototype/HighQualityMaleFolder/HumanMaleHighQualityAnimsFolder/Attack_anim_pass_3_Montage.Attack_anim_pass_3_Montage" :!type "AnimMontage Object Reference")))

(fn `UserConstructionScript`)