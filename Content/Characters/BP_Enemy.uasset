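; BP_Enemy is an enemy Blueprint that displays a health bar through a widget component.
; Every Tick, it casts the widget to BP_EnemyHPBar and sets the bar's percent from Health, assuming a 100-point maximum.
; It then rotates the widget component toward the player camera with a look-at rotation, skipping both updates if the cast fails.
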(event `self.ReceiveTick`
  (params (DeltaSeconds :type "Float (single-precision)"))
  (bind _health_bar_widget (`self.Health_Bar_Widget`))
  ;[1 1 1] Displays the healthbar ontop of the enemy and sets percentage of health bar to overall enemy health / 100 for 100 hp points
  (bind _asbp_enemy_hpbar (cast `/Game/UI/BP_EnemyHPBar` (`WidgetComponent.GetWidget` (`self.Health_Bar_Widget`))))
  (`ProgressBar.SetPercent` (`/Game/UI/BP_EnemyHPBar.EnemyHealthBar` _asbp_enemy_hpbar) (/ (`self.health`) 100.0))
  ;[1 1 1] Has healthbar following players camera rotation
  (`SceneComponent.K2_SetWorldRotation` _health_bar_widget (`KismetMathLibrary.FindLookAtRotation` (`SceneComponent.K2_GetComponentLocation` _health_bar_widget) (`SceneComponent.K2_GetComponentLocation` (`PlayerCameraManager.TransformComponent` (`GameplayStatics.GetPlayerCameraManager` 0)))) false false))

(fn `UserConstructionScript`)