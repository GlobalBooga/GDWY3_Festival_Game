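; Actor component that reads a custom hardware controller over a serial port and exposes its input as Forward and Right values.
; BeginPlay stores the owner, scans low-numbered COM ports, keeps the first that opens and flushes it.
; Tick reads a line and splits "D"-tagged comma-separated data into the two axes, with optional debug logging.
; EndPlay closes the port to release it.
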(event `self.ReceiveTick`
  (params (DeltaSeconds :type "Float (single-precision)"))
  (bind _debugstr (`self.DebugStr`))
  (bind (_lefts _rights) (`KismetStringLibrary.Split` (`KismetStringLibrary.Replace` _debugstr "D,") ","))
  ;[1 1 1] Parse data from serial port into data we can use
  (if (`self.IsSerialPortOpen`)
    (bind (_bsuccess _returnvalue) (`SerialCom.Readln` (`self.SerialPort`)))
    (bind _output_get (set `self.DebugStr` _returnvalue))
    (if _bsuccess
      (if (`KismetStringLibrary.Contains` _output_get "D")
        (if (`self.DebugLogging`)
          (`KismetSystemLibrary.PrintString` _debugstr))
        (set `self.right` (`KismetStringLibrary.Conv_StringToDouble` _lefts))
        (set `self.forward` (`KismetStringLibrary.Conv_StringToDouble` _rights))
        (elif (`self.DebugLogging`)
          (`KismetSystemLibrary.PrintString` _debugstr))))))

(event `self.ReceiveBeginPlay`
  ;[1 1 1] Set player reference then find a COM port
  (set `self.PlayerRef` (`self.GetOwner`))
  (for _index (range 11)
    (bind (_bopened _returnvalue) (`SerialCom.OpenComPortWithFlowControl` _index))
    (bind _output_get (set `self.IsSerialPortOpen` _bopened))
    (if _output_get
      (set `self.SerialPort` _returnvalue)
      (set `self.ComIndex` _index)
      (break)))
  (`SerialCom.Flush` (`self.SerialPort`))
  (if (and (`self.IsSerialPortOpen`) (`self.DebugLogging`))
    (`KismetSystemLibrary.PrintString` "Connected to port ")
    (`KismetSystemLibrary.PrintString` (`KismetStringLibrary.Conv_IntToString` (`self.ComIndex`)))))

(event `self.ReceiveEndPlay`
  (params (EndPlayReason :type "EEndPlayReason Enum" :default "Destroyed"))
  ;[1 1 1] IMPORTANT - close serial port on end play
  (if (`self.IsSerialPortOpen`)
    (`SerialCom.Close` (`self.SerialPort`))
    (set `self.IsSerialPortOpen` false)))